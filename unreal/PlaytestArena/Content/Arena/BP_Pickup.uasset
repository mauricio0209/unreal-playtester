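; BP_Pickup is a gem pickup that adds an amount to the inventory when the player touches it, then destroys itself.
; BeginPlay sets the Gem component to overlap all dynamic objects.
; On overlap with player 0's pawn, it finds BP_TestHarness via GetActorOfClass and passes Amount to its AddInventory.
; An unconnected copy of the pickup logic never runs, and Tick is unused.
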(event `self.ReceiveBeginPlay`
  (`PrimitiveComponent.SetCollisionProfileName` (`self.Gem`) "OverlapAllDynamic" true))

(event `self.ReceiveActorBeginOverlap`
  (params (OtherActor :type "Actor Object Reference"))
  (if (== OtherActor (`GameplayStatics.GetPlayerPawn` 0))
    (bind _returnvalue (`GameplayStatics.GetActorOfClass` "/Game/Harness/BP_TestHarness.BP_TestHarness_C"))
    (`/Game/Harness/BP_TestHarness.AddInventory` _returnvalue (`self.Amount`))
    (`self.K2_DestroyActor` self)))

(fn `UserConstructionScript`)