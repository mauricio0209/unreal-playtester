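; Playtest harness actor that keeps the game paused and advances it in timed, counted steps on demand.
; Exposes commands to move, jump, look, interact with doors, screenshot, switch camera and reload the level.
; Tick steers the pawn toward a 2D target and caches its last non-negative-Z location.
; GetState returns a snapshot of step, pawn, inventory, doors and pickups, using cached values when the pawn is gone.
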(event `self.ReceiveBeginPlay`
  (set `self.BootTime` (* (`KismetMathLibrary.RandomFloat`) 1000000.0))
  (bind _asbp_playtest_game_instance (cast `/Game/Harness/BP_PlaytestGameInstance` (`GameplayStatics.GetGameInstance`))
    (:`then`
      (set `/Game/Harness/BP_PlaytestGameInstance.LoadCount` (+ (`/Game/Harness/BP_PlaytestGameInstance.LoadCount` _asbp_playtest_game_instance) 1) _asbp_playtest_game_instance)
      (`GameplayStatics.SetGamePaused` true))
    (:`CastFailed`
      (`GameplayStatics.SetGamePaused` true))))

(event `self.ReceiveTick`
  (params (DeltaSeconds :type "Float (single-precision)"))
  (bind _returnvalue (`GameplayStatics.GetPlayerPawn` 0))
  (bind _movetarget (`self.MoveTarget`))
  (bind _returnvalue_2 (`self.K2_GetActorLocation` _returnvalue))
  (bind _returnvalue_3 (`KismetMathLibrary.MakeVector` (- (.x _movetarget) (.x _returnvalue_2)) (- (.y _movetarget) (.y _returnvalue_2))))
  (`/Engine/EditorBlueprintResources/StandardMacros.IsValid` _returnvalue
    (:`Is Valid`
      (set `self.LastZ` (.z _returnvalue_2))
      (if (>= (.z _returnvalue_2) 0.0)
        (set `self.LastLocation` _returnvalue_2))
      (if (`self.bHasMoveTarget`)
        (if (< (`KismetMathLibrary.VSize` _returnvalue_3) 50.0)
          (set `self.bHasMoveTarget` false)
          (else
            (`Pawn.AddMovementInput` _returnvalue (`KismetMathLibrary.Normal` _returnvalue_3) 1.0 false)))))))

(fn `AddInventory`
  (params (Amount :type Integer))
  (set `self.InventoryCount` (+ (`self.InventoryCount`) Amount)))

(fn `EndStep`
  (`GameplayStatics.SetGamePaused` true)
  (set `self.StepCounter` (+ (`self.StepCounter`) 1))
  (set `self.bStepActive` false))

(fn `GetState`
  (returns (StepId :type Integer) (bStepping :type Boolean) (PawnAlive :type Boolean) (PlayerLocation :type "Vector Structure") (Velocity :type "Vector Structure") (LastZ :type "Float (double-precision)") (KillZ :type "Float (double-precision)") (bIsFalling :type Boolean) (InventoryCount :type Integer) (BootTime :type "Float (double-precision)") (ActorStates :type "Map of String to String") (ActorLocations :type "Map of String to Vector Structure") (LastFloorLocation :type "Vector Structure"))
  (bind _returnvalue (`GameplayStatics.GetPlayerPawn` 0))
  (bind _stepcounter (`self.StepCounter`))
  (bind _bstepactive (`self.bStepActive`))
  (bind _inventorycount (`self.InventoryCount`))
  (bind _boottime (`self.BootTime`))
  (bind _trackedstates (`self.TrackedStates`))
  (bind _trackedlocations (`self.TrackedLocations`))
  (bind _lastlocation (`self.LastLocation`))
  (bind _returnvalue_2 (`self.K2_GetActorLocation` _returnvalue))
  (`BlueprintMapLibrary.Map_Clear` (`self.TrackedStates`))
  (`BlueprintMapLibrary.Map_Clear` (`self.TrackedLocations`))
  (bind _outactors (`GameplayStatics.GetAllActorsOfClass` "/Game/Arena/BP_Door.BP_Door_C"))
  (for _array_element _outactors
    (bind _returnvalue_3 (`KismetSystemLibrary.GetDisplayName` _array_element))
    (`BlueprintMapLibrary.Map_Add` (`self.TrackedStates`) _returnvalue_3 (select `bool` (`/Game/Arena/BP_Door.bOpen` _array_element) :`false` "closed" :`true` "open"))
    (`BlueprintMapLibrary.Map_Add` (`self.TrackedLocations`) _returnvalue_3 (`self.K2_GetActorLocation` _array_element)))
  (bind _outactors_2 (`GameplayStatics.GetAllActorsOfClass` "/Game/Arena/BP_Pickup.BP_Pickup_C"))
  (for _array_element_2 _outactors_2
    (bind _returnvalue_4 (`KismetSystemLibrary.GetDisplayName` _array_element_2))
    (`BlueprintMapLibrary.Map_Add` (`self.TrackedStates`) _returnvalue_4 "present")
    (`BlueprintMapLibrary.Map_Add` (`self.TrackedLocations`) _returnvalue_4 (`self.K2_GetActorLocation` _array_element_2)))
  (bind _returnvalue_5 (`GameplayStatics.GetActorOfClass` "/Script/Engine.WorldSettings"))
  (`/Engine/EditorBlueprintResources/StandardMacros.IsValid` _returnvalue
    (:`Is Valid`
      (bind _killz (`WorldSettings.KillZ` _returnvalue_5))
      (return _stepcounter _bstepactive true _returnvalue_2 (`self.GetVelocity` _returnvalue) (.z _returnvalue_2) _killz (`NavMovementInterface.IsFalling` (`Pawn.GetMovementComponent` _returnvalue)) _inventorycount _boottime _trackedstates _trackedlocations _lastlocation))
    (:`Is Not Valid`
      (return _stepcounter _bstepactive false _lastlocation (`KismetMathLibrary.Vector_Zero`) (`self.LastZ`) _killz false _inventorycount _boottime _trackedstates _trackedlocations _lastlocation))))

(fn `Interact`
  (bind _outactors (`GameplayStatics.GetAllActorsOfClass` "/Game/Arena/BP_Door.BP_Door_C"))
  (for _array_element _outactors
    (`/Game/Arena/BP_Door.TryInteract` _array_element (`GameplayStatics.GetPlayerPawn` 0))))

(fn `Jump`
  (bind _ascharacter (cast `Character` (`GameplayStatics.GetPlayerPawn` 0)))
  (`Character.Jump` _ascharacter)
  (`KismetSystemLibrary.K2_SetTimer` self "StopJump" 0.1))

(fn `LookAt`
  (params (X :type "Float (double-precision)") (Y :type "Float (double-precision)") (Z :type "Float (double-precision)"))
  (bind _returnvalue (`GameplayStatics.GetPlayerPawn` 0))
  (`/Engine/EditorBlueprintResources/StandardMacros.IsValid` _returnvalue
    (:`Is Valid`
      (`Controller.SetControlRotation` (`GameplayStatics.GetPlayerController` 0) (`KismetMathLibrary.FindLookAtRotation` (+ (`self.K2_GetActorLocation` _returnvalue) (`KismetMathLibrary.MakeVector` 0.0 0.0 60.0)) (`KismetMathLibrary.MakeVector` X Y Z))))))

(fn `MoveTo`
  (params (X :type "Float (double-precision)") (Y :type "Float (double-precision)"))
  (set `self.MoveTarget` (`KismetMathLibrary.MakeVector` X Y))
  (set `self.bHasMoveTarget` true))

(fn `ResetLevel`
  (bind _returnvalue (`GameplayStatics.GetCurrentLevelName` true))
  (`GameplayStatics.OpenLevel` (`KismetStringLibrary.Conv_StringToName` _returnvalue)))

(fn `Screenshot`
  (`KismetSystemLibrary.ExecuteConsoleCommand` "HighResShot 960x540" null))

(fn `SetCamera`
  (params (Mode :type String))
  (`KismetSystemLibrary.ExecuteConsoleCommand` (`KismetStringLibrary.Concat_StrStr` "camera " Mode) null))

(fn `Step`
  (params (Seconds :type "Float (double-precision)"))
  (set `self.bStepActive` true)
  (`GameplayStatics.SetGamePaused` false)
  (`KismetSystemLibrary.K2_SetTimer` self "EndStep" Seconds))

(fn `StopJump`
  (bind _ascharacter (cast `Character` (`GameplayStatics.GetPlayerPawn` 0)))
  (`Character.StopJumping` _ascharacter))

(fn `UserConstructionScript`)